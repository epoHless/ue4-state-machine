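; Enemy character that patrols waypoints, chases the player and flags an attack on arrival.
; A StateProcessorEnemyBehaviour receives CharacterMovement in construction; the file exposes movement events plus distance checks for engage and attack ranges.
; AIMoveTo drives both movement modes, with waypoint travel re-calling itself on success to continue along linked waypoints.
; AI Perception updates SeesPlayer, and Tick draws both ranges as debug spheres.
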(event `Reset Movement`
  ;[1 1 1] Stop Active Movement
  (`NavMovementComponent.StopActiveMovement` (`self.CharacterMovement`)))

(event `self.ReceiveBeginPlay`
  ;[1 1 1] Set Initial State
)

(event `self.ReceiveTick`
  (params (DeltaSeconds :type "Float (single-precision)"))
  ;[1 1 1] Draw Debug Circles
  (`KismetSystemLibrary.DrawDebugSphere` (`self.K2_GetActorLocation`) (`self.Engage Range`) 12 (struct :`R` 1.0 :`G` 0.827556 :`A` 1.0) 0.0 2.0)
  (`KismetSystemLibrary.DrawDebugSphere` (`self.K2_GetActorLocation`) (`self.Attack Range`) 12 (struct :`R` 1.0 :`A` 1.0) 0.0 2.0))

(event `self.AIPerception.OnTargetPerceptionUpdated`
  (params (Actor :type "Actor Object Reference") (Stimulus :type "AIStimulus Structure"))
  ;[1 1 1] Attack / Engage State
  (set `self.Sees Player` (`.bSuccessfullySensed` (break `AIStimulus` Stimulus))))

(event `Move To Waypoint`
  (params (Waypoint :type "Waypoint Object Reference"))
  ;[1 1 1] Move From One Waypoint To Another
  (`|AIMoveTo` self (0.0 0.0 0.0) (`Waypoint.GetNextWaypoint` Waypoint)
    (:`OnSuccess`
      (bind _returnvalue (`TravelerComponent.SetCurrentWaypoint` (`self.Traveler`) (`Waypoint.GetNextWaypoint` (`TravelerComponent.GetCurrentWaypoint` (`self.Traveler`)))))
      (`self.Move To Waypoint` _returnvalue))))

(event `Move To Player`
  ;[1 1 1] Move To Player Location
  (`|AIMoveTo` self (0.0 0.0 0.0) (`GameplayStatics.GetPlayerPawn` 0)
    (:`OnSuccess`
      (set `self.Attack` true))))

(fn `Should Attack?`
  (returns (ReturnValue :type Boolean))
  (return (<= (`KismetMathLibrary.Vector_Distance` (`self.K2_GetActorLocation`) (`self.K2_GetActorLocation` (`GameplayStatics.GetPlayerPawn` 0))) (`self.Attack Range`))))

(fn `Should Engage?`
  (returns (ReturnValue :type Boolean))
  (return (<= (`KismetMathLibrary.Vector_Distance` (`self.K2_GetActorLocation`) (`self.K2_GetActorLocation` (`GameplayStatics.GetPlayerPawn` 0))) (`self.Engage Range`))))

(fn `UserConstructionScript`
  (`AStateProcessor.SetController` (`self.StateProcessor_EnemyBehaviour`) (`self.CharacterMovement`)))